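; EnemyContext is an EQS query context that supplies a single enemy actor to environment queries run by robber AI.
; For a robber pawn, it returns the Enemy stored on its Robber_Controller.
; When the querier is an EQS testing pawn, it substitutes the first Ai_PoliceCharacter found in the level.
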(fn `ProvideSingleActor`
  (params (QuerierObject :type "Object Object Reference") (QuerierActor :type "Actor Object Reference"))
  (returns (ResultingActor :type "Actor Object Reference"))
  (locals (TempEnemy :type "Actor Object Reference"))
  (cast `EQSTestingPawn` QuerierActor
    (:`then`
      (bind _outactors (`GameplayStatics.GetAllActorsOfClass` "/Game/Blueprints/MattsStuff/AI/Ai_PoliceCharacter.Ai_PoliceCharacter_C"))
      (set `local.TempEnemy` (`KismetArrayLibrary.Array_Get` _outactors)))
    (:`CastFailed`
      (bind _returnvalue (`AIBlueprintHelperLibrary.GetAIController` QuerierActor))
      (if (!= _returnvalue null)
        (bind _asrobber_controller (cast `/Game/Blueprints/KeilsStuff/Robber_Controller` _returnvalue)
          (:`then`
            (set `local.TempEnemy` (`/Game/Blueprints/KeilsStuff/Robber_Controller.Enemy` _asrobber_controller)))
          (:`CastFailed`
            _)))))
  (return (`local.TempEnemy`)))