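; AI controller for a robber that runs the Robber_Tree behavior tree and tracks police as enemies.
; On begin play it starts the tree and, after a short delay, calls SetEnemy with the player pawn.
; AI Perception updates filter for Ai_PoliceCharacter actors and check their first sensed stimulus.
; The results feed the blackboard's enemy visibility and enemy object keys for the tree.
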(event `self.ReceiveBeginPlay`
  ;[1 1 1] grab enemy and put in behavior tree
  (`self.RunBehaviorTree` "/Game/Blueprints/KeilsStuff/Robber_Tree.Robber_Tree")
  (`KismetSystemLibrary.Delay` 1.0)
  (`self.SetEnemy` (`GameplayStatics.GetPlayerPawn` 0))
  (`BlackboardComponent.SetValueAsObject` (`AIBlueprintHelperLibrary.GetBlackboard` self) (`self.BlackboardKeyEnemy`) null))

(event `self.AIPerception.OnPerceptionUpdated`
  (params (UpdatedActors :type "Array of Actor Object Reference"))
  ;[1 1 1] set enemy to blackboard keys for behavior tree
  (`self.UpdateEnemyRecords` UpdatedActors))

(fn `SetEnemy`
  (params (NewEnemy :type "Actor Object Reference"))
  (if (!= NewEnemy (`self.Enemy`))
    (bind _output_get (set `self.Enemy` NewEnemy))
    (`BlackboardComponent.SetValueAsObject` (`AIBlueprintHelperLibrary.GetBlackboard` null) (`self.BlackboardKeyEnemy`) _output_get)))

(fn `UpdateEnemyRecords`
  (params (UpdatedActors :type "Array of Actor Object Reference"))
  (locals (HasSeenAnEnemy :type Boolean) (SeenEnemy :type "Object Object Reference"))
  (bind _returnvalue (`AIBlueprintHelperLibrary.GetBlackboard` self))
  (for _array_element UpdatedActors
    (bind _asai_police_character (cast `/Game/Blueprints/MattsStuff/AI/Ai_PoliceCharacter` _array_element)) ; Filter by PoliceCharacter\n\n(this is probably not necessary anymore)
    (bind _info (`AIPerceptionComponent.GetActorsPerception` (`self.AIPerception`) _asai_police_character)) ; Do a perception test
    ;[1 1 1] Update temporary recordkeeping for enemy percepts
    (bind _output_get (set `local.HasSeenAnEnemy` (or (`local.HasSeenAnEnemy`) (`.bSuccessfullySensed` (break `AIStimulus` (`KismetArrayLibrary.Array_Get` (`.LastSensedStimuli` (break `ActorPerceptionBlueprintInfo` _info))))))))
    (if _output_get
      (set `local.SeenEnemy` _asai_police_character)))
  (`|ExecutionSequence`
    (:`then_0`
      (`BlackboardComponent.SetValueAsBool` _returnvalue (`self.BlackboardKeyIsEnemyVisible`) (`local.HasSeenAnEnemy`)))
    (:`then_1`
      (`BlackboardComponent.SetValueAsObject` _returnvalue (`self.BlackboardKeyEnemy`) (`local.SeenEnemy`)))))

(fn `UserConstructionScript`)