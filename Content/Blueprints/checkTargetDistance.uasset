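; Behavior tree decorator for the police AI that checks how far its controlled pawn is from the target it follows.
; It casts the owner to the police AI controller, then reads the TargetToFollow actor from the blackboard.
; The condition passes when the straight-line distance between target and pawn is at least AcceptableDistance.
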(fn `PerformConditionCheck`
  (params (OwnerActor :type "Actor Object Reference"))
  (returns (ReturnValue :type Boolean))
  (bind _aspolice_ai_con (cast `/Game/Blueprints/Police_Ai_CON` OwnerActor))
  (set `self.AI_CON_Ref` _aspolice_ai_con)
  (return (>= (`KismetMathLibrary.VSize` (- (`Actor.K2_GetActorLocation` (`BTFunctionLibrary.GetBlackboardValueAsActor` (`self.TargetToFollow`))) (`Actor.K2_GetActorLocation` (`Controller.K2_GetPawn` (`self.AI_CON_Ref`))))) (`self.AcceptableDistance`))))